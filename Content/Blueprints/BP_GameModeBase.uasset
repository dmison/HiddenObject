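; BP_GameModeBase is a game mode that handles background ambiance and a score-based win condition.
; It creates and plays an ambiance audio component on BeginPlay and stops it on EndPlay.
; IncrementScore raises Score by one, and on reaching MaxScore sets GameOver and plays a short applause sound.
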(event `self.ReceiveBeginPlay`
  ;[1 1 1] Start playing background ambiance when game starts
  (bind _returnvalue (`AddComponent|NODE_AddAudioComponent-0`))
  (`AudioComponent.Play` _returnvalue 0.0))

(event `self.ReceiveEndPlay`
  (params (EndPlayReason :type "EEndPlayReason Enum" :default "Destroyed"))
  ;[1 1 1] Stop playing background ambiance when game ends
  (`AudioComponent.Stop` (stale `self.ReceiveBeginPlay` _returnvalue)))

(fn `Increment Score`
  ;[0.3763 0.2176 1] Increments the Score by one
  (bind _result (`/Engine/EditorBlueprintResources/StandardMacros.IncrementInt` (`self.Score`))
    (:`  `
      ;[0.653 0.5799 1] If score >= max score then set game over to true
      (if (>= _result (`self.MaxScore`))
        (set `self.bGameOver` true)
        (`GameplayStatics.PlaySound2D` "/Game/Audio/241132__xtrgamr__shortapplause_01.241132__xtrgamr__shortapplause_01" 1.0 1.0 0.0 null null)))))

(fn `UserConstructionScript`)